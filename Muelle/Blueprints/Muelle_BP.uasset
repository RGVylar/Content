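; Spring pad Blueprint for a 2D side-scroller that bounces the player character upward on contact.
; When its Box is overlapped, it switches the flipbook to the spring animation and launches the 2DSideScrollerCharacter with the Impulso value as vertical velocity, overriding Z.
; When the overlap ends, it waits half a second, restores the idle flipbook and calls a zero-velocity, non-overriding launch on the character.
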(event `self.Box.OnComponentBeginOverlap`
  (params (OverlappedComponent :type "PrimitiveComponent Object Reference") (OtherActor :type "Actor Object Reference") (OtherComp :type "PrimitiveComponent Object Reference") (OtherBodyIndex :type Integer) (bFromSweep :type Boolean) (SweepResult :type "HitResult Structure (by ref)"))
  ;[1 1 1] Para propulsar y animar el muelle
  (`PaperFlipbookComponent.SetFlipbook` (`self.PaperFlipbook`) "/Game/Muelle/Animaciones/MuelleAnim.MuelleAnim")
  (bind _as2dside_scroller_character (cast `/Game/Personaje/Blueprints/2DSideScrollerCharacter` OtherActor))
  (`Character.LaunchCharacter` _as2dside_scroller_character (`KismetMathLibrary.MakeVector` 0.0 0.0 (`self.Impulso`)) false true))

(event `self.Box.OnComponentEndOverlap`
  (params (OverlappedComponent :type "PrimitiveComponent Object Reference") (OtherActor :type "Actor Object Reference") (OtherComp :type "PrimitiveComponent Object Reference") (OtherBodyIndex :type Integer))
  ;[1 1 1] Para dejar de propulsar y animar el muelle
  (`KismetSystemLibrary.Delay` 0.5)
  (`PaperFlipbookComponent.SetFlipbook` (`self.PaperFlipbook`) "/Game/Muelle/Animaciones/IdleMuelle.IdleMuelle")
  (bind _as2dside_scroller_character (cast `/Game/Personaje/Blueprints/2DSideScrollerCharacter` OtherActor))
  (`Character.LaunchCharacter` _as2dside_scroller_character (0.0 0.0 0.0) false false))

(fn `UserConstructionScript`)