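; Enemy bot for a 2D side-scroller that spots, chases and catches the player, tinted a random color at spawn.
; Tick uses player distance to forget or spot them (quack and message), then chase along X, jumping when they are higher.
; At close range it stops chasing, and when nearly touching sets the player's End flag.
; While chasing, UpdateAnimation swaps body and hand flipbooks by movement state; the crouch trigger is unconnected.
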(event `UpdateAnimation`
  (bind _paperflipbook1 (`self.PaperFlipbook1`))
  (bind _paperflipbook (`self.PaperFlipbook`))
  (bind _sprite (`self.Sprite`))
  (bind _agachado (`self.agachado`))
  (bind _quack (`self.Quack`))
  ;[1 1 1] Handle Animation
  (bind _output_get (set `self.moviendose` (== (`KismetMathLibrary.VSize` (`self.GetVelocity`)) 0.0)))
  (if _output_get
    (if _agachado
      (`PaperFlipbookComponent.SetFlipbook` _sprite (select `bool` _quack :`false` "/Game/2DSideScroller/Sprites/CrouchAnimation_Bot.CrouchAnimation_Bot" :`true` "/Game/Personaje/Animaciones/CrouchAnimation_Quack.CrouchAnimation_Quack" :!type "PaperFlipbook Object Reference"))
      (`PaperFlipbookComponent.SetFlipbook` _paperflipbook "/Game/Personaje/Animaciones/Idle_Hands.Idle_Hands")
      (`PaperFlipbookComponent.SetFlipbook` _paperflipbook1 "/Game/Personaje/Animaciones/Idle_Hands.Idle_Hands")
      (else
        (`PaperFlipbookComponent.SetFlipbook` _sprite (select `bool` _quack :`false` "/Game/2DSideScroller/Sprites/IdleAnimation_Bot.IdleAnimation_Bot" :`true` "/Game/2DSideScroller/Sprites/IdleAnimation_Quack.IdleAnimation_Quack" :!type "PaperFlipbook Object Reference"))
        (`PaperFlipbookComponent.SetFlipbook` _paperflipbook "/Game/Personaje/Animaciones/Idle_Hands.Idle_Hands")
        (`PaperFlipbookComponent.SetFlipbook` _paperflipbook1 "/Game/Personaje/Animaciones/Idle_Hands.Idle_Hands")))
    (elif _agachado
      (`PaperFlipbookComponent.SetFlipbook` _sprite (select `bool` _quack :`false` "/Game/2DSideScroller/Sprites/CrouchAnimation_Bot.CrouchAnimation_Bot" :`true` "/Game/2DSideScroller/Sprites/CrouchingMov_Quack.CrouchingMov_Quack" :!type "PaperFlipbook Object Reference"))
      (`PaperFlipbookComponent.SetFlipbook` _paperflipbook "/Game/Personaje/Animaciones/Idle_Hands.Idle_Hands")
      (`PaperFlipbookComponent.SetFlipbook` _paperflipbook1 "/Game/Personaje/Animaciones/Idle_Hands.Idle_Hands")
      (elif (`self.saltando`)
        (`PaperFlipbookComponent.SetFlipbook` _sprite (select `bool` _quack :`false` "/Game/2DSideScroller/Sprites/JumpingAnimation_Bot.JumpingAnimation_Bot" :`true` "/Game/2DSideScroller/Sprites/JumpingAnimation_Quack.JumpingAnimation_Quack" :!type "PaperFlipbook Object Reference"))
        (`PaperFlipbookComponent.SetFlipbook` _paperflipbook "/Game/Personaje/Animaciones/Jump_hand.Jump_hand")
        (`PaperFlipbookComponent.SetFlipbook` _paperflipbook1 "/Game/Personaje/Animaciones/Jump_hand.Jump_hand")
        (else
          (`PaperFlipbookComponent.SetFlipbook` _sprite (select `bool` _quack :`false` "/Game/2DSideScroller/Sprites/RunningAnimation_Bot.RunningAnimation_Bot" :`true` "/Game/2DSideScroller/Sprites/RunningAnimation_Quack.RunningAnimation_Quack" :!type "PaperFlipbook Object Reference"))
          (`PaperFlipbookComponent.SetFlipbook` _paperflipbook "/Game/Personaje/Animaciones/Running_hands.Running_hands")
          (`PaperFlipbookComponent.SetFlipbook` _paperflipbook1 "/Game/Personaje/Animaciones/Running_hands.Running_hands"))))))

(event `self.ReceiveTick`
  (params (DeltaSeconds :type "Float (single-precision)"))
  (bind _returnvalue (`self.K2_GetActorLocation`))
  (bind _paperflipbook2 (`self.PaperFlipbook2`))
  (bind _sprite (`self.Sprite`))
  (bind _returnvalue_2 (`self.K2_GetActorLocation` (`GameplayStatics.GetPlayerCharacter` 0)))
  (bind _returnvalue_3 (`KismetMathLibrary.VSize` (- _returnvalue_2 _returnvalue)))
  (bind _returnvalue_4 (> (.x _returnvalue_2) (.x _returnvalue)))
  ;[1 1 1] Tick - Updates animation
  (if (> _returnvalue_3 1000.0)
    (set `self.visto` false)
    (elif (<= _returnvalue_3 200.0)
      (`PaperFlipbookComponent.SetFlipbook` _paperflipbook2 null)
      (set `self.girando` true)
      (if (`self.girando`)
        (if (<= _returnvalue_3 95.0)
          ;[1 1 1] Handle movement
          (bind _as2dside_scroller_character (cast `/Game/Personaje/Blueprints/2DSideScrollerCharacter` (`GameplayStatics.GetPlayerPawn` 0)))
          (set `/Game/Personaje/Blueprints/2DSideScrollerCharacter.End` true _as2dside_scroller_character)
          (`self.SetActorHiddenInGame` _as2dside_scroller_character false)))
      (else
        (`PaperFlipbookComponent.SetFlipbook` _paperflipbook2 null)
        (if (`self.visto`)
          (`self.UpdateAnimation`)
          (`/Engine/EditorBlueprintResources/StandardMacros.CompareFloat` (.x (`MovementComponent.Velocity` (`self.GetMovementComponent`)))
            (:`>`
              (`SceneComponent.K2_SetWorldRotation` _sprite (`KismetMathLibrary.MakeRotator` 0.0) false false :!label _label)
              (`SceneComponent.K2_SetWorldRotation` (`self.PaperFlipbook`) (`KismetMathLibrary.MakeRotator` 0.0) false false)
              (`SceneComponent.K2_SetWorldRotation` (`self.espada`) (`KismetMathLibrary.MakeRotator` 0.0) false false))
            (:`==`
              (if _returnvalue_4
                (goto _label)
                (else
                  (`SceneComponent.K2_SetWorldRotation` _sprite (`KismetMathLibrary.MakeRotator` 0.0 0.0 180.0) false false :!label _label_2)
                  (`SceneComponent.K2_SetWorldRotation` (`self.PaperFlipbook`) (`KismetMathLibrary.MakeRotator` 0.0 0.0 180.0) false false)
                  (`SceneComponent.K2_SetWorldRotation` (`self.espada`) (`KismetMathLibrary.MakeRotator` 0.0 0.0 180.0) false false))))
            (:`<`
              (goto _label_2)))
          (if (not (<= _returnvalue_3 95.0))
            (if _returnvalue_4
              (`self.AddMovementInput` (10.0 0.0 0.0))
              (else
                ;[1 1 1] Handle Jump
                (`self.AddMovementInput` (-10.0 0.0 0.0))))
            (if (> (.z _returnvalue_2) (.z _returnvalue))
              (`self.Jump`)
              (set `self.saltando` true)
              (`KismetSystemLibrary.Delay` 1.0)
              (set `self.saltando` false)
              (`self.StopJumping`)))
          (else
            (bind _output_get (set `self.visto` (< _returnvalue_3 1000.0)))
            (if _output_get
              (`KismetSystemLibrary.PrintString` "Te ví!" true true (select `int` (`KismetMathLibrary.RandomInteger` 2) :`0` (select `int` (`KismetMathLibrary.RandomInteger` 2) :`0` (select `int` (`KismetMathLibrary.RandomInteger` 2) :`0` (struct :`R` 1.0 :`G` 0.556642 :`A` 1.0) :`1` (struct :`R` 1.0 :`G` 1.0 :`B` 1.0 :`A` 1.0) :!type "LinearColor Structure") :`1` (select `int` (`KismetMathLibrary.RandomInteger` 2) :`0` (struct :`R` 1.0 :`B` 0.961659 :`A` 1.0) :`1` (struct :`G` 0.982318 :`B` 1.0 :`A` 1.0) :!type "LinearColor Structure")) :`1` (select `int` (`KismetMathLibrary.RandomInteger` 2) :`0` (select `int` (`KismetMathLibrary.RandomInteger` 2) :`0` (struct :`R` 1.0 :`A` 1.0) :`1` (struct :`G` 0.160882 :`B` 1.0 :`A` 1.0) :!type "LinearColor Structure") :`1` (select `int` (`KismetMathLibrary.RandomInteger` 2) :`0` (struct :`G` 1.0 :`B` 0.024281 :`A` 1.0) :`1` (struct :`R` 1.0 :`G` 0.95954 :`A` 1.0) :!type "LinearColor Structure"))))
              (set `self.Quack` true)
              (`GameplayStatics.PlaySound2D` "/Game/2DSideScroller/Sprites/QuackDucks/quack-normal.quack-normal")
              (`KismetSystemLibrary.Delay` 5.0)
              (set `self.Quack` false))))))))

(event `self.ReceiveBeginPlay`
  (bind _sprite (`self.Sprite`))
  (`ActorComponent.SetIsReplicated` _sprite true)
  (`ActorComponent.SetIsReplicated` (`self.PaperFlipbook`) true)
  (`self.EnableInput` null)
  ;[1 1 1] Tick - Updates animation
  (`PaperFlipbookComponent.SetSpriteColor` _sprite (select `int` (`KismetMathLibrary.RandomInteger` 2) :`0` (select `int` (`KismetMathLibrary.RandomInteger` 2) :`0` (select `int` (`KismetMathLibrary.RandomInteger` 2) :`0` (struct :`R` 1.0 :`G` 0.556642 :`A` 1.0) :`1` (struct :`R` 1.0 :`G` 1.0 :`B` 1.0 :`A` 1.0) :!type "LinearColor Structure") :`1` (select `int` (`KismetMathLibrary.RandomInteger` 2) :`0` (struct :`R` 1.0 :`B` 0.961659 :`A` 1.0) :`1` (struct :`G` 0.982318 :`B` 1.0 :`A` 1.0) :!type "LinearColor Structure")) :`1` (select `int` (`KismetMathLibrary.RandomInteger` 2) :`0` (select `int` (`KismetMathLibrary.RandomInteger` 2) :`0` (struct :`R` 1.0 :`A` 1.0) :`1` (struct :`G` 0.160882 :`B` 1.0 :`A` 1.0) :!type "LinearColor Structure") :`1` (select `int` (`KismetMathLibrary.RandomInteger` 2) :`0` (struct :`G` 1.0 :`B` 0.024281 :`A` 1.0) :`1` (struct :`R` 1.0 :`G` 0.95954 :`A` 1.0) :!type "LinearColor Structure"))))
  (`PaperFlipbookComponent.SetSpriteColor` (`self.PaperFlipbook`) (select `int` (`KismetMathLibrary.RandomInteger` 2) :`0` (select `int` (`KismetMathLibrary.RandomInteger` 2) :`0` (select `int` (`KismetMathLibrary.RandomInteger` 2) :`0` (struct :`R` 1.0 :`G` 0.556642 :`A` 1.0) :`1` (struct :`R` 1.0 :`G` 1.0 :`B` 1.0 :`A` 1.0) :!type "LinearColor Structure") :`1` (select `int` (`KismetMathLibrary.RandomInteger` 2) :`0` (struct :`R` 1.0 :`B` 0.961659 :`A` 1.0) :`1` (struct :`G` 0.982318 :`B` 1.0 :`A` 1.0) :!type "LinearColor Structure")) :`1` (select `int` (`KismetMathLibrary.RandomInteger` 2) :`0` (select `int` (`KismetMathLibrary.RandomInteger` 2) :`0` (struct :`R` 1.0 :`A` 1.0) :`1` (struct :`G` 0.160882 :`B` 1.0 :`A` 1.0) :!type "LinearColor Structure") :`1` (select `int` (`KismetMathLibrary.RandomInteger` 2) :`0` (struct :`G` 1.0 :`B` 0.024281 :`A` 1.0) :`1` (struct :`R` 1.0 :`G` 0.95954 :`A` 1.0) :!type "LinearColor Structure"))))
  (`PaperFlipbookComponent.SetSpriteColor` (`self.PaperFlipbook1`) (select `int` (`KismetMathLibrary.RandomInteger` 2) :`0` (select `int` (`KismetMathLibrary.RandomInteger` 2) :`0` (select `int` (`KismetMathLibrary.RandomInteger` 2) :`0` (struct :`R` 1.0 :`G` 0.556642 :`A` 1.0) :`1` (struct :`R` 1.0 :`G` 1.0 :`B` 1.0 :`A` 1.0) :!type "LinearColor Structure") :`1` (select `int` (`KismetMathLibrary.RandomInteger` 2) :`0` (struct :`R` 1.0 :`B` 0.961659 :`A` 1.0) :`1` (struct :`G` 0.982318 :`B` 1.0 :`A` 1.0) :!type "LinearColor Structure")) :`1` (select `int` (`KismetMathLibrary.RandomInteger` 2) :`0` (select `int` (`KismetMathLibrary.RandomInteger` 2) :`0` (struct :`R` 1.0 :`A` 1.0) :`1` (struct :`G` 0.160882 :`B` 1.0 :`A` 1.0) :!type "LinearColor Structure") :`1` (select `int` (`KismetMathLibrary.RandomInteger` 2) :`0` (struct :`G` 1.0 :`B` 0.024281 :`A` 1.0) :`1` (struct :`R` 1.0 :`G` 0.95954 :`A` 1.0) :!type "LinearColor Structure")))))

(fn `UserConstructionScript`)