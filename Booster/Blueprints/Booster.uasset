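; Booster actor that carries the side-scroller player between two points when they enter its trigger Box.
; On overlap it sets the character's Saltando (jumping) flag and clears Activo, then plays a timeline from the start.
; The timeline lerps the player's location from Scene1 to Scene, teleporting without sweep.
; Leaving the Box stops the timeline but does not restore either flag.
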(event `self.Box.OnComponentBeginOverlap`
  (params (OverlappedComponent :type "PrimitiveComponent Object Reference") (OtherActor :type "Actor Object Reference") (OtherComp :type "PrimitiveComponent Object Reference") (OtherBodyIndex :type Integer) (bFromSweep :type Boolean) (SweepResult :type "HitResult Structure (by ref)"))
  (bind _returnvalue (`GameplayStatics.GetPlayerCharacter` 0))
  (bind _as2dside_scroller_character (cast `/Game/Personaje/Blueprints/2DSideScrollerCharacter` _returnvalue :!pure true))
  (if (== OtherActor _returnvalue)
    (set `/Game/Personaje/Blueprints/2DSideScrollerCharacter.saltando` true _as2dside_scroller_character)
    (set `/Game/Personaje/Blueprints/2DSideScrollerCharacter.Activo` false _as2dside_scroller_character)
    (bind (_direction _newtrack_0) (`Timeline|Timeline_0` :!via `PlayFromStart` :!label _label)
      (:`Update`
        (`self.K2_SetActorLocation` _as2dside_scroller_character (`KismetMathLibrary.VLerp` (`SceneComponent.K2_GetComponentLocation` (`self.Scene1`)) (`SceneComponent.K2_GetComponentLocation` (`self.Scene`)) _newtrack_0) false true)))))

(event `self.Box.OnComponentEndOverlap`
  (params (OverlappedComponent :type "PrimitiveComponent Object Reference") (OtherActor :type "Actor Object Reference") (OtherComp :type "PrimitiveComponent Object Reference") (OtherBodyIndex :type Integer))
  (if (== (`GameplayStatics.GetPlayerCharacter` 0) OtherActor)
    (goto _label :!via `Stop`)))

(fn `UserConstructionScript`)