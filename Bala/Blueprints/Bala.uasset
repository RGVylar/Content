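; Bala is a bullet projectile that kills Bot actors on hit and can end the game when it strikes the player.
; On collision it loops over every Bot; a match is destroyed with a death sound, and a black-tinted Ragdoll replaces the bullet at its transform.
; Non-matching iterations reach a short delay, then flag End on the side-scroller character if the player was hit.
; Weapon cast and Inicio Patos counter nodes are unconnected.
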(event `self.CollisionComponent.OnComponentHit`
  (params (HitComponent :type "PrimitiveComponent Object Reference") (OtherActor :type "Actor Object Reference") (OtherComp :type "PrimitiveComponent Object Reference") (NormalImpulse :type "Vector Structure") (Hit :type "HitResult Structure (by ref)"))
  (bind _outactors (`GameplayStatics.GetAllActorsOfClass` "/Game/Bot/Blueprints/Bot.Bot_C"))
  (for _array_element _outactors
    (if (== _array_element OtherActor)
      (set `self.body` (`self.GetTransform`))
      (`KismetSystemLibrary.PrintString` (`KismetSystemLibrary.GetDisplayName` OtherActor))
      (`self.K2_DestroyActor` OtherActor)
      (`GameplayStatics.PlaySound2D` "/Game/2DSideScroller/Sounds/death.death" 2.0)
      (`self.K2_DestroyActor`)
      (bind _returnvalue (`|SpawnActorFromClass` "/Game/Ragdoll/Blueprints/Ragdoll.Ragdoll_C" (`self.body`) "AlwaysSpawn" "OverrideRootScale" null null))
      (`PaperSpriteComponent.SetSpriteColor` (`/Game/Ragdoll/Blueprints/Ragdoll.Centro` _returnvalue) (struct :`A` 1.0))
      (`PaperSpriteComponent.SetSpriteColor` (`/Game/Ragdoll/Blueprints/Ragdoll.Patas` _returnvalue) (struct :`A` 1.0))
      (`PaperSpriteComponent.SetSpriteColor` (`/Game/Ragdoll/Blueprints/Ragdoll.Cabeza` _returnvalue) (struct :`A` 1.0))
      (else
        (`KismetSystemLibrary.Delay` 0.2)
        (if (== OtherActor (`GameplayStatics.GetPlayerCharacter` 0))
          (set `/Game/Personaje/Blueprints/2DSideScrollerCharacter.End` true (cast `/Game/Personaje/Blueprints/2DSideScrollerCharacter` (`GameplayStatics.GetPlayerPawn` 0) :!pure true))
          (`self.SetActorHiddenInGame` OtherActor false))))))

(fn `UserConstructionScript`)