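; Short-lived explosion actor that removes a bot caught in its box or switches the camera when it catches the player.
; BeginPlay waits briefly, then checks the actor from the box's begin-overlap event, whose own execution path is empty.
; A matching Bot is destroyed, while the player character triggers a view-target switch to the first Capture_2 actor.
; The explosion then destroys itself.
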(event `self.ReceiveBeginPlay`
  (`KismetSystemLibrary.Delay` 0.2)
  (if (!= (`GameplayStatics.GetPlayerCharacter` 0) (stale `self.Box.OnComponentBeginOverlap` OtherActor))
    (if (== (stale `self.Box.OnComponentBeginOverlap` OtherActor) "/Game/2DSideScrollerBP/Blueprints/Bot.Bot")
      (`self.K2_DestroyActor` (stale `self.Box.OnComponentBeginOverlap` OtherActor)))
    (else
      (bind _outactors (`GameplayStatics.GetAllActorsOfClass` "/Game/2DSideScrollerBP/Blueprints/Camera/Capture_2.Capture_2_C"))
      (`PlayerController.SetViewTargetWithBlend` (`GameplayStatics.GetPlayerController` 0) (`|GetArrayItem` _outactors) 0.0 "VTBlend_Linear" 0.0 false)))
  (`self.K2_DestroyActor`))

(event `self.Box.OnComponentBeginOverlap`
  (params (OverlappedComponent :type "PrimitiveComponent Object Reference") (OtherActor :type "Actor Object Reference") (OtherComp :type "PrimitiveComponent Object Reference") (OtherBodyIndex :type Integer) (bFromSweep :type Boolean) (SweepResult :type "HitResult Structure (by ref)")))

(fn `UserConstructionScript`)