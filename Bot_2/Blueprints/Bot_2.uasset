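; AI-controlled 2D Paper2D bot that roams toward targets, grabs weapons and shoots what it detects ahead.
; Overlapping a Weapon_BP while unarmed attaches it; when armed, Tick line-traces in the facing direction and fires after a delay.
; Otherwise Tick seeks the nearest Objetivo_BP, flips sprites and weapon, and uses traces to jump obstacles and intended gaps.
; UpdateAnimation swaps body and hand flipbooks by movement state and Quack/Bot skin; crouch logic is unconnected.
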(event `self.CapsuleComponent.OnComponentEndOverlap`
  (params (OverlappedComponent :type "PrimitiveComponent Object Reference") (OtherActor :type "Actor Object Reference") (OtherComp :type "PrimitiveComponent Object Reference") (OtherBodyIndex :type Integer))
  ;[1 1 1] Coger Arma
  (if (== OtherActor (`self.Arma`))
    (set `self.Armado` false)))

(event `self.CapsuleComponent.OnComponentBeginOverlap`
  (params (OverlappedComponent :type "PrimitiveComponent Object Reference") (OtherActor :type "Actor Object Reference") (OtherComp :type "PrimitiveComponent Object Reference") (OtherBodyIndex :type Integer) (bFromSweep :type Boolean) (SweepResult :type "HitResult Structure (by ref)"))
  ;[1 1 1] Coger Arma
  (if (`self.Armado`)
    (`KismetSystemLibrary.PrintString` "Aqui hay un arma!" true true (struct :`R` 1.0 :`G` 0.811921 :`A` 1.0)) ; Si estoy armado indico al jugador que hay un arma
    (else
      (`self.GrabGun` OtherActor OtherActor) ; Si no estoy armado cojo el arma
    )))

(event `UpdateAnimation`
  ;[1 1 1] Animar
  (bind _output_get (set `self.moviendose` (== (`KismetMathLibrary.VSize` (`self.GetVelocity`)) 0.0)))
  (if _output_get
    (if (`self.agachado`)
      (`PaperFlipbookComponent.SetFlipbook` (`self.Sprite`) (select `bool` (`self.Quack`) :`false` "/Game/2DSideScroller/Sprites/CrouchAnimation_Bot.CrouchAnimation_Bot" :`true` "/Game/Personaje/Animaciones/CrouchAnimation_Quack.CrouchAnimation_Quack" :!type "PaperFlipbook Object Reference"))
      (`PaperFlipbookComponent.SetFlipbook` (`self.PaperFlipbook`) "/Game/Personaje/Animaciones/Idle_Hands.Idle_Hands")
      (`PaperFlipbookComponent.SetFlipbook` (`self.PaperFlipbook1`) "/Game/Personaje/Animaciones/Idle_Hands.Idle_Hands")
      (else
        (`PaperFlipbookComponent.SetFlipbook` (`self.Sprite`) (select `bool` (`self.Quack`) :`false` "/Game/2DSideScroller/Sprites/CrouchingMov_Bot.CrouchingMov_Bot" :`true` "/Game/2DSideScroller/Sprites/CrouchingMov_Quack.CrouchingMov_Quack" :!type "PaperFlipbook Object Reference"))
        (`PaperFlipbookComponent.SetFlipbook` (`self.PaperFlipbook`) "/Game/Personaje/Animaciones/Idle_Hands.Idle_Hands")
        (`PaperFlipbookComponent.SetFlipbook` (`self.PaperFlipbook1`) "/Game/Personaje/Animaciones/Idle_Hands.Idle_Hands")))
    (elif (`self.agachado`)
      (`PaperFlipbookComponent.SetFlipbook` (`self.Sprite`) (select `bool` (`self.Quack`) :`false` "/Game/2DSideScroller/Sprites/CrouchAnimation_Bot.CrouchAnimation_Bot" :`true` "/Game/2DSideScroller/Sprites/CrouchingMov_Quack.CrouchingMov_Quack" :!type "PaperFlipbook Object Reference"))
      (`PaperFlipbookComponent.SetFlipbook` (`self.PaperFlipbook`) "/Game/Personaje/Animaciones/Idle_Hands.Idle_Hands")
      (`PaperFlipbookComponent.SetFlipbook` (`self.PaperFlipbook1`) "/Game/Personaje/Animaciones/Idle_Hands.Idle_Hands")
      (elif (`self.saltando`)
        (`PaperFlipbookComponent.SetFlipbook` (`self.Sprite`) (select `bool` (`self.Quack`) :`false` "/Game/2DSideScroller/Sprites/JumpingAnimation_Bot.JumpingAnimation_Bot" :`true` "/Game/2DSideScroller/Sprites/JumpingAnimation_Quack.JumpingAnimation_Quack" :!type "PaperFlipbook Object Reference"))
        (`PaperFlipbookComponent.SetFlipbook` (`self.PaperFlipbook`) "/Game/Personaje/Animaciones/Jump_hand.Jump_hand")
        (`PaperFlipbookComponent.SetFlipbook` (`self.PaperFlipbook1`) "/Game/Personaje/Animaciones/Jump_hand.Jump_hand")
        (else
          (`PaperFlipbookComponent.SetFlipbook` (`self.Sprite`) (select `bool` (`self.Quack`) :`false` "/Game/2DSideScroller/Sprites/RunningAnimation_Bot.RunningAnimation_Bot" :`true` "/Game/2DSideScroller/Sprites/RunningAnimation_Quack.RunningAnimation_Quack" :!type "PaperFlipbook Object Reference"))
          (`PaperFlipbookComponent.SetFlipbook` (`self.PaperFlipbook`) "/Game/Personaje/Animaciones/Running_hands.Running_hands")
          (`PaperFlipbookComponent.SetFlipbook` (`self.PaperFlipbook1`) "/Game/Personaje/Animaciones/Running_hands.Running_hands"))))))

(event `self.ReceiveBeginPlay`
  ;[1 1 1] Preparar Bot
  (`ActorComponent.SetIsReplicated` (`self.Sprite`) true))

(event `self.ReceiveTick`
  (params (DeltaSeconds :type "Float (single-precision)"))
  (bind _loc (`self.Loc`))
  (bind _x (.x (`self.Loc`)))
  (bind _y (.y (`self.Loc`)))
  (bind _z (.z (`self.Loc`)))
  (bind _returnvalue (`KismetMathLibrary.VSize` (- (`self.Objetivo`) _loc)))
  (bind _returnvalue_2 (+ (.x (`self.Loc`)) 200.0))
  ;[1 1 1] Comprobar Ubicacion y Equipacion
  (set `self.Loc` (`self.K2_GetActorLocation`))
  (if (`self.Armado`)
    ;[1 1 1] Comprobar si es enemigo
    (bind _outhit (`KismetSystemLibrary.LineTraceSingleForObjects` (`self.Loc`) (`KismetMathLibrary.MakeVector` (`KismetMathLibrary.SelectFloat` (+ _x 300.0) (- _x 300.0) (`self.direccion`)) (.y (`self.Loc`)) (.z (`self.Loc`))) (`|MakeArray` "ObjectTypeQuery4" :!type "EObjectTypeQuery Enum") false (`|MakeArray` (`self.Arma`)) "ForOneFrame")) ; Hago un ray trace desde mi localizacion hasta 300 pixels hacia donde mire
    ;[1 1 1] Disparar
    (if (`GameplayStatics.BreakHitResult` _outhit)
      (`KismetSystemLibrary.Delay` 1.0)
      (`/Game/Weapon/Blueprints/Weapon_BP.Disparar` (`self.Arma`))
      (else
        ;[1 1 1] Buscar Objetivos
        (bind _outactors (`GameplayStatics.GetAllActorsOfClass` "/Game/Objetivo/Objetivo_BP.Objetivo_BP_C" :!label _label))
        (for _array_element _outactors
          ;[1 1 1] Decidir Objetivo cercano
          (set `self.Al Lado` (<= _returnvalue 95.0)) ; Si estoy al lado, detengo el movimiento
          (bind _returnvalue_3 (`self.K2_GetActorLocation` _array_element))
          ;[1 1 1] Reconocer Obstaculos
          (if (not (> (`KismetMathLibrary.VSize` (- _returnvalue_3 _loc)) _returnvalue))
            (set `self.Objetivo` _returnvalue_3))
          (bind _outhit_2 (`KismetSystemLibrary.LineTraceSingleForObjects` :`Start` (`self.Loc`) :`End` (`KismetMathLibrary.MakeVector` _returnvalue_2 _y _z) :`ObjectTypes` (`|MakeArray` "ObjectTypeQuery3" :!type "EObjectTypeQuery Enum") :`DrawDebugType` "ForOneFrame" :`TraceColor` (struct :`R` 0.010704 :`B` 1.0 :`A` 1.0) :`TraceHitColor` (struct :`G` 0.9599 :`B` 1.0 :`A` 1.0))) ; Mientras me muevo voy buscano obstaculos
          (bind _outhit_3 (`KismetSystemLibrary.LineTraceSingleForObjects` :`Start` (`self.Loc`) :`End` (`KismetMathLibrary.MakeVector` _returnvalue_2 _y (/ _z 2.0)) :`ObjectTypes` (`|MakeArray` "ObjectTypeQuery3" :!type "EObjectTypeQuery Enum") :`DrawDebugType` "ForOneFrame" :`TraceColor` (struct :`G` 0.700115 :`B` 1.0 :`A` 1.0) :`TraceHitColor` (struct :`G` 0.057209 :`B` 1.0 :`A` 1.0))) ; Tambien busco agujeros
          (`self.UpdateAnimation`) ; Envio señal para cambiar mi animacion
          (set `self.direccion` (> (.x (`self.Objetivo`)) (.x (`self.Loc`))))
          (set `self.Vacio` (`GameplayStatics.BreakHitResult` _outhit_3)) ; Hay un hueco
          (set `self.Pared` (`GameplayStatics.BreakHitResult` _outhit_2)) ; Hay un obstaculo
          ;[1 1 1] Cambiar Rotacion
          (`/Engine/EditorBlueprintResources/StandardMacros.CompareFloat` (.x (`MovementComponent.Velocity` (`self.GetMovementComponent`)))
            (:`>`
              (`SceneComponent.K2_SetWorldRotation` :`self` (`self.PaperFlipbook`) :!label _label_2)
              (`SceneComponent.K2_SetWorldRotation` :`self` (`self.Sprite`))
              (`/Engine/EditorBlueprintResources/StandardMacros.IsValid` null ; Compruebo si tengo un arma antes de girarla
                (:`Is Valid`
                  (`SceneComponent.K2_SetWorldRotation` :`self` (`Actor.RootComponent` (`self.Arma`))))
                (:`Is Not Valid`
                  _)))
            (:`==`
              (if (`self.direccion`)
                (goto _label_2)
                (else
                  (`SceneComponent.K2_SetWorldRotation` (`self.Sprite`) (struct :`Yaw` 180.0) false false :!label _label_3)
                  (`SceneComponent.K2_SetWorldRotation` (`self.PaperFlipbook`) (struct :`Yaw` 180.0) false false)
                  (`/Engine/EditorBlueprintResources/StandardMacros.IsValid` null
                    (:`Is Valid`
                      (`SceneComponent.K2_SetWorldRotation` (`Actor.RootComponent` (`self.Arma`)) (struct :`Yaw` 180.0) false false))
                    (:`Is Not Valid`
                      _)))))
            (:`<`
              (goto _label_3)))
          ;[1 1 1] Moverse hacia el objetivo
          (if (`self.Al Lado`)
            (set `self.Objetivo` (* (`self.Objetivo`) -1)) ; Si esta al lado, su objetivo cambia a un lejano, porque si no, no vuelve a irse a ningun otro objetivo, ya que el que esta al aldo es el mas cercano!
            (else
              (if (`self.direccion`)
                (`self.AddMovementInput` (10.0 0.0 0.0)) ; Puedo variar la velocidad con una variable en la direccion, que contenga un valor mayor o menor al actual
                (else
                  (`self.AddMovementInput` (-10.0 0.0 0.0))))
              ;[1 1 1] Evitar obstaculos
              (if (`self.Pared`)
                (`self.Jump` :!label _label_4)
                (set `self.saltando` true)
                (`KismetSystemLibrary.Delay` 0.2) ; Mantengo el salto un poco para que la animacion se muestre como quiero
                (set `self.saltando` false)
                (`self.StopJumping`)
                (elif (`self.Vacio`)
                  (goto _label_4)
                  (else
                    (`KismetSystemLibrary.Delay` 5.0)
                    (set `self.Objetivo` (1000.0 1000.0 1000.0)) ; Si esta al lado, su objetivo cambia a un lejano, porque si no, no vuelve a irse a ningun otro objetivo, ya que el que esta al aldo es el mas cercano!
                  ))))))))
    (else
      (goto _label))))

(fn `CogerArma`
  (params (B :type "Object Object Reference")))

(fn `GrabGun`
  (params (Object :type "Object Object Reference") (Object2 :type "Object Object Reference"))
  ;[1 1 1] Apropiarse del Arma
  (if (== (`GameplayStatics.GetObjectClass` Object) "/Game/Weapon/Blueprints/Weapon_BP.Weapon_BP_C")
    (bind _output_get (set `self.Arma` (cast `/Game/Weapon/Blueprints/Weapon_BP` Object2 :!pure true))) ; Meto el arma en la variable Arma
    ;[1 1 1] Adaptar Arma
    (`PrimitiveComponent.SetEnableGravity` (`/Game/Weapon/Blueprints/Weapon_BP.PaperSprite2` _output_get) false) ; Le quito la gravedad para evitarme problemas
    (`self.K2_AttachToActor` (`self.Arma`) self "None" "SnapToTarget" "KeepRelative" "KeepRelative" true) ; De esta manera el arma se mantiene en mi ubicacion
    (set `self.Armado` true) ; Estoy armado
  ))

(fn `UserConstructionScript`)