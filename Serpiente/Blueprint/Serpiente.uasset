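; Snake (Serpiente) 2D character that moves in step with the player's horizontal direction.
; Tick looks up all 2DSideScrollerCharacter actors, and a BeginPlay timeline reads the first one's BisMovingRight flag to apply movement input along its track vector or the negated vector.
; Each update sets the Serpiente2 flipbook and restarts a yaw-flip timeline, whose rotation lerp reads the other flip timeline's track.
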(event `self.ReceiveBeginPlay`
  (bind _paperflipbook (`self.PaperFlipbook`))
  (bind (_direction _newtrack_0) (`Timeline|Timeline_0`)
    (:`Update`
      (bind _output (`|GetArrayItem` (stale `self.ReceiveTick` _outactors)))
      (if (`KismetSystemLibrary.IsValid` _output)
        (`PaperFlipbookComponent.SetFlipbook` (`self.PaperFlipbook`) "/Game/Boxes/Texturas/Serpiente2.Serpiente2")
        (if (`/Game/Personaje/Blueprints/2DSideScrollerCharacter.bisMovingRight` _output)
          (`self.AddMovementInput` _newtrack_0)
          (bind (_direction_2 _newtrack_0_2) (`Timeline|Timeline_2` :!via `PlayFromStart`)
            (:`Update`
              (`SceneComponent.K2_SetRelativeRotation` _paperflipbook (`KismetMathLibrary.MakeRotator` 0.0 0.0 (`KismetMathLibrary.Lerp` 0.0 180.0 (stale _newtrack_0_3))) false false)))
          (else
            (`self.AddMovementInput` (`KismetMathLibrary.NegateVector` _newtrack_0))
            (bind (_direction_3 _newtrack_0_3) (`Timeline|Timeline_1` :!via `PlayFromStart`)
              (:`Update`
                (`SceneComponent.K2_SetRelativeRotation` _paperflipbook (`KismetMathLibrary.MakeRotator` 0.0 0.0 (`KismetMathLibrary.Lerp` 180.0 0.0 _newtrack_0_2)) false false)))))))))

(event `self.ReceiveTick`
  (params (DeltaSeconds :type "Float (single-precision)"))
  (bind _outactors (`GameplayStatics.GetAllActorsOfClass` "/Game/Personaje/Blueprints/2DSideScrollerCharacter.2DSideScrollerCharacter_C")))

(fn `UserConstructionScript`)