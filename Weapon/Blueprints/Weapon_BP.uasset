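; Weapon Blueprint that randomly becomes one of two weapon types on BeginPlay, each with its own Paper2D sprite and magazine size.
; Pressing V calls Disparar, which spawns a Bala at the weapon's transform, decrements ammo and plays a shot sound.
; Firing with an empty magazine prints a message and destroys the weapon with a sound.
; An unconnected branch would increment a shot counter on the Inicio actor.
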(event `self.ReceiveBeginPlay`
  ;[1 1 1] Preparar Arma
  (set `self.Sprite` (`KismetMathLibrary.RandomInteger` 2)) ; Con el elijo que arma es
  (bind _output_get (set `self.Cargador` (select `int` (`self.Sprite`) :`0` 8 :`1` 30))) ; Elijo su cargador
  (set `self.Balas` _output_get) ; Relleno las balas
  (`PaperSpriteComponent.SetSprite` (`self.PaperSprite2`) (select `int` (`self.Sprite`) :`0` null :`1` null :!type "PaperSprite Object Reference")) ; Pongo el sprite del arma adecuada
)

(event `Key|V`
  (params (Key :type "Key Structure"))
  ;[1 1 1] Disparar
  (:`Pressed`
    (`self.Disparar`) ; Ejecuto el disparo
  ))

(fn `Disparar`
  ;[1 1 1] Comprobar Municion
  (if (> (`self.Balas`) 0)
    ;[1 1 1] Generar Bala
    (`|SpawnActorFromClass` "/Game/Bala/Blueprints/Bala.Bala_C" (`self.GetTransform` self) "Undefined" "OverrideRootScale" null null)
    ;[1 1 1] Estadisticas
    (bind _result (`/Engine/EditorBlueprintResources/StandardMacros.DecrementInt` (`self.Balas`)) ; Resto una bala a mi municion
      (:`  `
        (bind _output_get (set `self.Balas` _result))
        (`KismetSystemLibrary.PrintString` (`KismetStringLibrary.Conv_IntToString` _output_get))
        (`GameplayStatics.PlaySound2D` "/Game/2DSideScroller/Sounds/magnum.magnum") ; Reproduzco el sonido del disparo
      ))
    (else
      ;[1 1 1] Desechar Arma
      (`KismetSystemLibrary.PrintString` "Sin balas") ; Si no hay balas, lo comunico
      (`self.K2_DestroyActor`) ; Elimino el arma vacia
      (`GameplayStatics.PlaySound2D` "/Game/2DSideScroller/Sounds/ignite.ignite" 2.0) ; Reproduzco un sonido de destruccion
    )))

(fn `UserConstructionScript`)