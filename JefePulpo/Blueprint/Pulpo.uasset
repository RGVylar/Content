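; Octopus boss (Pulpo) for a 2D side-scroller that moves, spawns Gota actors and can kill the player.
; Overlapping Box starts a timeline-driven movement whose direction depends on the player's side.
; Tick uses a Delay to spawn a Gota every second, then yaws the flipbook by player facing via two timelines reading each other's tracks.
; Matar overlap ends and hides the player; RestarVida subtracts damage, destroying the boss at zero health.
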(event `self.Box.OnComponentBeginOverlap`
  (params (OverlappedComponent :type "PrimitiveComponent Object Reference") (OtherActor :type "Actor Object Reference") (OtherComp :type "PrimitiveComponent Object Reference") (OtherBodyIndex :type Integer) (bFromSweep :type Boolean) (SweepResult :type "HitResult Structure (by ref)"))
  (if (== (`GameplayStatics.GetPlayerCharacter` 0) OtherActor)
    (bind (_direction _newtrack_0) (`Timeline|Timeline_0`)
      (:`Update`
        (bind _output (`|GetArrayItem` (stale `self.ReceiveTick` _outactors)))
        (if (`KismetSystemLibrary.IsValid` _output)
          (if (> (.x (`self.K2_GetActorLocation` _output)) (.x (`self.K2_GetActorLocation`)))
            (`self.AddMovementInput` _newtrack_0)
            (else
              (`self.AddMovementInput` (`KismetMathLibrary.NegateVector` _newtrack_0)))))))))

(event `self.ReceiveTick`
  (params (DeltaSeconds :type "Float (single-precision)"))
  (bind _paperflipbook (`self.PaperFlipbook`))
  (bind _posicion (`self.Posicion`))
  (bind _outactors (`GameplayStatics.GetAllActorsOfClass` "/Game/Personaje/Blueprints/2DSideScrollerCharacter.2DSideScrollerCharacter_C"))
  (`KismetSystemLibrary.Delay` 1.0)
  (bind _returnvalue (`|SpawnActorFromClass` "/Game/Gota/Blueprint/Gota.Gota_C" (`KismetMathLibrary.MakeTransform` (`KismetMathLibrary.MakeVector` (+ (.x (.location (`self.GetTransform`))) _posicion) 0.0 (+ (.z (.location (`self.GetTransform`))) _posicion)) (struct) (0.2 1.0 0.2)) "Undefined" "OverrideRootScale" null null))
  (set `/Game/Gota/Blueprint/Gota.Zpulpo` (.z (`self.K2_GetActorLocation`)) _returnvalue)
  (if (`/Game/Personaje/Blueprints/2DSideScrollerCharacter.bisMovingRight` (`|GetArrayItem` _outactors))
    (bind (_direction _newtrack_0) (`Timeline|Timeline_2`)
      (:`Update`
        (`SceneComponent.K2_SetRelativeRotation` _paperflipbook (`KismetMathLibrary.MakeRotator` 0.0 0.0 (`KismetMathLibrary.Lerp` 0.0 180.0 (stale _newtrack_0_2))) false false)))
    (else
      (bind (_direction_2 _newtrack_0_2) (`Timeline|Timeline_1`)
        (:`Update`
          (`SceneComponent.K2_SetRelativeRotation` _paperflipbook (`KismetMathLibrary.MakeRotator` 0.0 0.0 (`KismetMathLibrary.Lerp` 180.0 0.0 _newtrack_0)) false false))))))

(event `self.Matar.OnComponentBeginOverlap`
  (params (OverlappedComponent :type "PrimitiveComponent Object Reference") (OtherActor :type "Actor Object Reference") (OtherComp :type "PrimitiveComponent Object Reference") (OtherBodyIndex :type Integer) (bFromSweep :type Boolean) (SweepResult :type "HitResult Structure (by ref)"))
  (if (== OtherActor (`GameplayStatics.GetPlayerCharacter` 0))
    (set `/Game/Personaje/Blueprints/2DSideScrollerCharacter.End` true (cast `/Game/Personaje/Blueprints/2DSideScrollerCharacter` (`GameplayStatics.GetPlayerPawn` 0) :!pure true))
    (`self.SetActorHiddenInGame` OtherActor true)))

(fn `RestarVida`
  (bind _output_get (set `self.Vida` (- (`self.Vida`) (`self.Daño`))))
  (if (<= _output_get 0)
    (`self.K2_DestroyActor`)
    (`KismetSystemLibrary.PrintString` (`KismetStringLibrary.Conv_IntToString` _output_get))))

(fn `UserConstructionScript`)