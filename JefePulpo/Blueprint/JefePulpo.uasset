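; JefePulpo is an octopus boss character that moves along X and spawns Gota (drop) actors.
; Tick plays a timeline whose track drives LaunchCharacter; on finish, it spawns a Gota at an X offset.
; After a delay it destroys the drop, updates the offset, then destroys itself through an always-true comparison.
; RestarVida subtracts damage from health and destroys the boss at zero or below.
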(event `self.ReceiveTick`
  (params (DeltaSeconds :type "Float (single-precision)"))
  (bind (_direction _newtrack_1) (`Timeline|Timeline_0`)
    (:`Update`
      (`self.LaunchCharacter` (`KismetMathLibrary.MakeVector` _newtrack_1)))
    (:`Finished`
      (bind _returnvalue (`|SpawnActorFromClass` "/Game/2DSideScroller/Sprites/enemigos/gota.gota_C" (`KismetMathLibrary.Conv_VectorToTransform` (`KismetMathLibrary.MakeVector` (+ (.x (.location (`self.GetTransform`))) (`self.Posicion`)) (.y (.location (`self.GetTransform`))) (.z (.location (`self.GetTransform`))))) "Undefined" "OverrideRootScale" null null))
      (bind _output_get (set `self.Gota` _returnvalue))
      (`KismetSystemLibrary.Delay` 6.0)
      (`self.K2_DestroyActor` _output_get)
      (bind _result (`/Engine/EditorBlueprintResources/StandardMacros.NegateFloat` (`self.Posicion`))
        (:`  `
          (set `self.Posicion` _result)
          (if (== 0.0 0.0)
            (`self.K2_DestroyActor`)))))))

(fn `RestarVida`
  (bind _output_get (set `self.Vida` (- (`self.Vida`) (`self.Daño`))))
  (if (<= _output_get 0)
    (`self.K2_DestroyActor`)))

(fn `UserConstructionScript`)