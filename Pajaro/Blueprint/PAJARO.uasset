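; PAJARO is a bird hazard for the side-scroller that reacts to the player and can kill them.
; Entering BOX plays the bird sound and starts a timeline that launches the bird along Z using its track value each update.
; Touching the Matar volume sets End on the player's 2DSideScrollerCharacter and hides the player.
; RestarVida subtracts Daño from Vida with debug prints, destroying the bird at zero or below.
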(event `self.BOX.OnComponentBeginOverlap`
  (params (OverlappedComponent :type "PrimitiveComponent Object Reference") (OtherActor :type "Actor Object Reference") (OtherComp :type "PrimitiveComponent Object Reference") (OtherBodyIndex :type Integer) (bFromSweep :type Boolean) (SweepResult :type "HitResult Structure (by ref)"))
  (if (== (`GameplayStatics.GetPlayerCharacter` 0) OtherActor)
    (`GameplayStatics.PlaySound2D` "/Game/Pajaro/Sonidos/Pajaro.Pajaro")
    (bind (_direction _newtrack_1) (`Timeline|Timeline_0`)
      (:`Update`
        (`self.LaunchCharacter` (`KismetMathLibrary.MakeVector` 0.0 0.0 _newtrack_1))))))

(event `self.Matar.OnComponentBeginOverlap`
  (params (OverlappedComponent :type "PrimitiveComponent Object Reference") (OtherActor :type "Actor Object Reference") (OtherComp :type "PrimitiveComponent Object Reference") (OtherBodyIndex :type Integer) (bFromSweep :type Boolean) (SweepResult :type "HitResult Structure (by ref)"))
  (if (== OtherActor (`GameplayStatics.GetPlayerCharacter` 0))
    (set `/Game/Personaje/Blueprints/2DSideScrollerCharacter.End` true (cast `/Game/Personaje/Blueprints/2DSideScrollerCharacter` (`GameplayStatics.GetPlayerPawn` 0) :!pure true))
    (`self.SetActorHiddenInGame` OtherActor true)))

(fn `RestarVida`
  (`KismetSystemLibrary.PrintString` "Recibo daño")
  (bind _output_get (set `self.Vida` (- (`self.Vida`) (`self.Daño`))))
  (if (<= _output_get 0)
    (`self.K2_DestroyActor`)
    (else
      (`KismetSystemLibrary.PrintString` (`KismetStringLibrary.Conv_IntToString` _output_get)))))

(fn `UserConstructionScript`)