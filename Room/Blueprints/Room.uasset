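; Room actor that shows a configurable Paper2D sprite and tracks whether the player is inside it.
; On BeginPlay it applies its Sprite variable to the PaperSprite component.
; Box overlap begin and end events, filtered to player character 0, set and clear the Activa flag.
; Both events then tint the sprite green while active and red when inactive.
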(event `self.ReceiveBeginPlay`
  (`PaperSpriteComponent.SetSprite` (`self.PaperSprite`) (`self.Sprite`)))

(event `self.Box.OnComponentBeginOverlap`
  (params (OverlappedComponent :type "PrimitiveComponent Object Reference") (OtherActor :type "Actor Object Reference") (OtherComp :type "PrimitiveComponent Object Reference") (OtherBodyIndex :type Integer) (bFromSweep :type Boolean) (SweepResult :type "HitResult Structure (by ref)"))
  (if (== OtherActor (`GameplayStatics.GetPlayerCharacter` 0))
    (set `self.Activa` true)
    (`PaperSpriteComponent.SetSpriteColor` (`self.PaperSprite`) (`KismetMathLibrary.SelectColor` (struct :`G` 1.0 :`A` 1.0) (struct :`R` 1.0 :`A` 1.0) (stale `self.Box.OnComponentEndOverlap` _output_get)) :!label _label)))

(event `self.Box.OnComponentEndOverlap`
  (params (OverlappedComponent :type "PrimitiveComponent Object Reference") (OtherActor :type "Actor Object Reference") (OtherComp :type "PrimitiveComponent Object Reference") (OtherBodyIndex :type Integer))
  (if (== (`GameplayStatics.GetPlayerCharacter` 0) OtherActor)
    (bind _output_get (set `self.Activa` false))
    (goto _label)))

(fn `UserConstructionScript`)