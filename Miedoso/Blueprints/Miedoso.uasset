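; Miedoso is a 2D side-scroller enemy that attacks or flees depending on whether the player character moves right.
; A Box overlap starts a timeline that drives movement, flipbook, sound and yaw flips, each flip timeline reading the other's track.
; Tick refetches the character list every frame for that direction check.
; Touching Matar flags the player's End and hides them, while RestarVida subtracts damage and destroys Miedoso at zero health.
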(event `self.Box.OnComponentBeginOverlap`
  (params (OverlappedComponent :type "PrimitiveComponent Object Reference") (OtherActor :type "Actor Object Reference") (OtherComp :type "PrimitiveComponent Object Reference") (OtherBodyIndex :type Integer) (bFromSweep :type Boolean) (SweepResult :type "HitResult Structure (by ref)"))
  (bind _paperflipbook (`self.PaperFlipbook`))
  (bind (_direction _newtrack_0) (`Timeline|Timeline_0`)
    (:`Update`
      (bind _output (`|GetArrayItem` (stale `self.ReceiveTick` _outactors)))
      (if (`KismetSystemLibrary.IsValid` _output)
        (if (`/Game/Personaje/Blueprints/2DSideScrollerCharacter.bisMovingRight` _output)
          (`self.AddMovementInput` _newtrack_0)
          (`PaperFlipbookComponent.SetFlipbook` (`self.PaperFlipbook`) "/Game/Miedoso/Texturas/MiedosoAtaca.MiedosoAtaca")
          (`GameplayStatics.PlaySound2D` "/Game/Miedoso/Sonidos/jejeje.jejeje")
          (bind (_direction_2 _newtrack_0_2) (`Timeline|Timeline_2` :!via `PlayFromStart`)
            (:`Update`
              (`SceneComponent.K2_SetRelativeRotation` _paperflipbook (`KismetMathLibrary.MakeRotator` 0.0 0.0 (`KismetMathLibrary.Lerp` 0.0 180.0 (stale _newtrack_0_3))) false false)))
          (else
            (`self.AddMovementInput` (`KismetMathLibrary.NegateVector` _newtrack_0))
            (`PaperFlipbookComponent.SetFlipbook` (`self.PaperFlipbook`) "/Game/Miedoso/Texturas/MiedosoHuye.MiedosoHuye")
            (`GameplayStatics.PlaySound2D` "/Game/Miedoso/Sonidos/Llorar.Llorar")
            (bind (_direction_3 _newtrack_0_3) (`Timeline|Timeline_1` :!via `PlayFromStart`)
              (:`Update`
                (`SceneComponent.K2_SetRelativeRotation` _paperflipbook (`KismetMathLibrary.MakeRotator` 0.0 0.0 (`KismetMathLibrary.Lerp` 180.0 0.0 _newtrack_0_2)) false false)))))))))

(event `self.ReceiveTick`
  (params (DeltaSeconds :type "Float (single-precision)"))
  (bind _outactors (`GameplayStatics.GetAllActorsOfClass` "/Game/Personaje/Blueprints/2DSideScrollerCharacter.2DSideScrollerCharacter_C")))

(event `self.Matar.OnComponentBeginOverlap`
  (params (OverlappedComponent :type "PrimitiveComponent Object Reference") (OtherActor :type "Actor Object Reference") (OtherComp :type "PrimitiveComponent Object Reference") (OtherBodyIndex :type Integer) (bFromSweep :type Boolean) (SweepResult :type "HitResult Structure (by ref)"))
  (if (== OtherActor (`GameplayStatics.GetPlayerCharacter` 0))
    (set `/Game/Personaje/Blueprints/2DSideScrollerCharacter.End` true (cast `/Game/Personaje/Blueprints/2DSideScrollerCharacter` (`GameplayStatics.GetPlayerPawn` 0) :!pure true))
    (`self.SetActorHiddenInGame` OtherActor true)))

(fn `RestarVida`
  (bind _output_get (set `self.Vida` (- (`self.Vida`) (`self.Daño`))))
  (if (<= _output_get 0)
    (`self.K2_DestroyActor`)))

(fn `UserConstructionScript`)