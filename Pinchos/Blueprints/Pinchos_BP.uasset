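; Spike hazard Blueprint (Pinchos) for a 2D side-scroller, displayed as a Paper2D flipbook.
; Overlap on R sets End on the player character and hides it, or destroys the overlapping actor if it is a Bot_2.
; The Final flag turns an instance into a gold-tinted variant that prints a loading message and opens the Start level after a short delay on player overlap.
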(event `self.ReceiveBeginPlay`
  (bind _paperflipbook (`self.PaperFlipbook`))
  (`PaperFlipbookComponent.SetFlipbook` _paperflipbook "/Game/Pinchos/Animaciones/Pinchos_FP.Pinchos_FP")
  (if (`self.Final`)
    (`PaperFlipbookComponent.SetSpriteColor` _paperflipbook (struct :`R` 1.0 :`G` 0.736161 :`A` 1.0))))

(event `self.R.OnComponentBeginOverlap`
  (params (OverlappedComponent :type "PrimitiveComponent Object Reference") (OtherActor :type "Actor Object Reference") (OtherComp :type "PrimitiveComponent Object Reference") (OtherBodyIndex :type Integer) (bFromSweep :type Boolean) (SweepResult :type "HitResult Structure (by ref)"))
  (if (== OtherActor (`GameplayStatics.GetPlayerCharacter` 0))
    (if (`self.Final`)
      (`KismetSystemLibrary.PrintString` "Cargando!")
      (`KismetSystemLibrary.Delay` 0.1)
      (`GameplayStatics.OpenLevel` "Start")
      (else
        (set `/Game/Personaje/Blueprints/2DSideScrollerCharacter.End` true (cast `/Game/Personaje/Blueprints/2DSideScrollerCharacter` (`GameplayStatics.GetPlayerPawn` 0) :!pure true))
        (`self.SetActorHiddenInGame` OtherActor true)))
    (else
      (bind _outactors (`GameplayStatics.GetAllActorsOfClass` "/Game/Bot_2/Blueprints/Bot_2.Bot_2_C"))
      (if (`KismetArrayLibrary.Array_IsValidIndex` _outactors)
        (for _array_element _outactors
          (if (== OtherActor _array_element)
            (`self.K2_DestroyActor` OtherActor)))))))

(fn `UserConstructionScript`)