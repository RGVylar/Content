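; Gotas is a Paper2D drop hazard that splashes on overlap and ends the run for the 2D side-scroller player it hits.
; It switches to the airborne flipbook half a second after BeginPlay.
; Any overlap on Explotar swaps in the collision flipbook and destroys the drop two seconds later.
; A separate Matar overlap sets the character's End flag and hides it, only for the player character.
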(event `self.ReceiveBeginPlay`
  (`KismetSystemLibrary.Delay` 0.5)
  (`PaperFlipbookComponent.SetFlipbook` (`self.PaperFlipbook`) "/Game/2DSideScroller/Sprites/enemigos/Gota/gota_air.gota_air"))

(event `self.Explotar.OnComponentBeginOverlap`
  (params (OverlappedComponent :type "PrimitiveComponent Object Reference") (OtherActor :type "Actor Object Reference") (OtherComp :type "PrimitiveComponent Object Reference") (OtherBodyIndex :type Integer) (bFromSweep :type Boolean) (SweepResult :type "HitResult Structure (by ref)"))
  (`PaperFlipbookComponent.SetFlipbook` (`self.PaperFlipbook`) "/Game/2DSideScroller/Sprites/enemigos/Gota/gota_collision.gota_collision")
  (`KismetSystemLibrary.Delay` 2.0)
  (`self.K2_DestroyActor`))

(event `self.Matar.OnComponentBeginOverlap`
  (params (OverlappedComponent :type "PrimitiveComponent Object Reference") (OtherActor :type "Actor Object Reference") (OtherComp :type "PrimitiveComponent Object Reference") (OtherBodyIndex :type Integer) (bFromSweep :type Boolean) (SweepResult :type "HitResult Structure (by ref)"))
  (if (== OtherActor (`GameplayStatics.GetPlayerCharacter` 0))
    (set `/Game/Personaje/Blueprints/2DSideScrollerCharacter.End` true (cast `/Game/Personaje/Blueprints/2DSideScrollerCharacter` (`GameplayStatics.GetPlayerPawn` 0) :!pure true))
    (`self.SetActorHiddenInGame` OtherActor true)))

(fn `UserConstructionScript`)