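; Gota is a Paper2D falling drop hazard that ends the run for the 2D side-scroller player on contact.
; A Delay inside Tick paces the fall into half-second downward steps, switching to the airborne flipbook when Cambiar is set.
; On reaching the Zpulpo height it shows the collision flipbook, then destroys itself after a short delay.
; Its Box overlap sets the character's End flag and hides the player.
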(event `self.ReceiveTick`
  (params (DeltaSeconds :type "Float (single-precision)"))
  (bind _paperflipbook (`self.PaperFlipbook`))
  (`KismetSystemLibrary.Delay` 0.5)
  (if (`self.Cambiar`)
    (`PaperFlipbookComponent.SetFlipbook` _paperflipbook "/Game/2DSideScroller/Sprites/enemigos/Gota/gota_air.gota_air")
    (set `self.Cambiar` false))
  (`self.K2_SetActorLocation` (`KismetMathLibrary.MakeVector` (.x (`self.K2_GetActorLocation`)) (.y (`self.K2_GetActorLocation`)) (- (.z (`self.K2_GetActorLocation`)) 50.0)))
  (if (<= (.z (`self.K2_GetActorLocation`)) (`self.Zpulpo`))
    (`PaperFlipbookComponent.SetFlipbook` _paperflipbook "/Game/2DSideScroller/Sprites/enemigos/Gota/gota_collision.gota_collision")
    (`KismetSystemLibrary.Delay` 1.0)
    (`self.K2_DestroyActor`)))

(event `self.Box.OnComponentBeginOverlap`
  (params (OverlappedComponent :type "PrimitiveComponent Object Reference") (OtherActor :type "Actor Object Reference") (OtherComp :type "PrimitiveComponent Object Reference") (OtherBodyIndex :type Integer) (bFromSweep :type Boolean) (SweepResult :type "HitResult Structure (by ref)"))
  (if (== OtherActor (`GameplayStatics.GetPlayerCharacter` 0))
    (set `/Game/Personaje/Blueprints/2DSideScrollerCharacter.End` true (cast `/Game/Personaje/Blueprints/2DSideScrollerCharacter` (`GameplayStatics.GetPlayerPawn` 0) :!pure true))
    (`self.SetActorHiddenInGame` OtherActor true)))

(fn `UserConstructionScript`)