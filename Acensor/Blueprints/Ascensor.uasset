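; Elevator actor that moves a sprite and its trigger box between the Inicio and Fin points.
; When Libres is set, the Libre timeline drives the motion from BeginPlay and overlaps are ignored.
; Otherwise, entering the box plays the Fija timeline and leaving reverses it, with the sprite tinted green or red by the Activo flag.
; Both timelines feed Animar, which lerps the world location without sweeping.
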(event `self.ReceiveBeginPlay`
  (if (`self.Libres`)
    (bind (_direction _newtrack_0) (`Timeline|Libre`)
      (:`Update`
        (`self.Animar` _newtrack_0)))))

(event `self.Box.OnComponentBeginOverlap`
  (params (OverlappedComponent :type "PrimitiveComponent Object Reference") (OtherActor :type "Actor Object Reference") (OtherComp :type "PrimitiveComponent Object Reference") (OtherBodyIndex :type Integer) (bFromSweep :type Boolean) (SweepResult :type "HitResult Structure (by ref)"))
  (if (not (`self.Libres`))
    (set `self.Activo` true)
    (bind (_direction _newtrack_0) (`Timeline|Fija` :!label _label)
      (:`Update`
        (`self.Animar` _newtrack_0)
        (`PaperSpriteComponent.SetSpriteColor` (`self.PaperSprite`) (`KismetMathLibrary.SelectColor` (struct :`G` 1.0 :`A` 1.0) (struct :`R` 1.0 :`A` 1.0) (`self.Activo`)))))))

(event `self.Box.OnComponentEndOverlap`
  (params (OverlappedComponent :type "PrimitiveComponent Object Reference") (OtherActor :type "Actor Object Reference") (OtherComp :type "PrimitiveComponent Object Reference") (OtherBodyIndex :type Integer))
  (if (not (`self.Libres`))
    (set `self.Activo` false)
    (goto _label :!via `Reverse`)))

(fn `Animar`
  (params (InputPin :type "Float (double-precision)"))
  (`SceneComponent.K2_SetWorldLocation` (`self.PaperSprite`) (`KismetMathLibrary.VLerp` (`SceneComponent.K2_GetComponentLocation` (`self.Inicio`)) (`SceneComponent.K2_GetComponentLocation` (`self.Fin`)) InputPin) false false)
  (`SceneComponent.K2_SetWorldLocation` (`self.Box`) (`KismetMathLibrary.VLerp` (`SceneComponent.K2_GetComponentLocation` (`self.Inicio`)) (`SceneComponent.K2_GetComponentLocation` (`self.Fin`)) InputPin) false false))

(fn `UserConstructionScript`)