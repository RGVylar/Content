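; Weapon actor that randomly picks one of two magazine sizes on BeginPlay, apparently revolver or AK, and fires on the V key while Sujeto is set.
; Each shot spawns a Bala at the world origin, decrements and prints the ammo, and plays a gunshot sound.
; Firing when empty prints a warning, destroys the weapon and plays another sound.
; The Dispara trigger, Inicio shot counter and sprite selection are unconnected.
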(event `self.ReceiveBeginPlay`
  (set `self.Arma` (`KismetMathLibrary.RandomInteger` 2))
  (bind _output_get (set `self.Cargador` (select `int` (`self.Arma`) :`0` 8 :`1` 30)))
  (set `self.Balas` _output_get))

(event `Key|V`
  (params (Key :type "Key Structure"))
  (bind _balas (`self.Balas`))
  (:`Pressed`
    (if (`self.Sujeto`)
      (if (> _balas 0)
        (`|SpawnActorFromClass` "/Game/Bala/Blueprints/Bala.Bala_C" (`KismetMathLibrary.MakeTransform` (0.0 0.0 0.0)) "Undefined" "OverrideRootScale" null null)
        (bind _result (`/Engine/EditorBlueprintResources/StandardMacros.DecrementInt` _balas)
          (:`  `
            (bind _output_get (set `self.Balas` _result))
            (`KismetSystemLibrary.PrintString` (`KismetStringLibrary.Conv_IntToString` _output_get))
            (`GameplayStatics.PlaySound2D` "/Game/2DSideScroller/Sounds/magnum.magnum")))
        (else
          (`KismetSystemLibrary.PrintString` "Sin balas")
          (`self.K2_DestroyActor`)
          (`GameplayStatics.PlaySound2D` "/Game/2DSideScroller/Sounds/ignite.ignite" 2.0))))))

(fn `UserConstructionScript`)