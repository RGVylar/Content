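; Pasillo_BP is a corridor piece for a 2D side-scroller that generates a room when the player character reaches it.
; When the 2DSideScrollerCharacter overlaps its Box trigger, it spawns a Habitacion_BP at a fixed X offset from the PaperSprite22 component.
; It then prints a debug message and destroys the Box, so each corridor generates only one room.
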(event `self.Box.OnComponentBeginOverlap`
  (params (OverlappedComponent :type "PrimitiveComponent Object Reference") (OtherActor :type "Actor Object Reference") (OtherComp :type "PrimitiveComponent Object Reference") (OtherBodyIndex :type Integer) (bFromSweep :type Boolean) (SweepResult :type "HitResult Structure (by ref)"))
  (cast `/Game/2DSideScrollerBP/Blueprints/2DSideScrollerCharacter` OtherActor)
  (`|SpawnActorFromClass` "/Game/2DSideScrollerBP/Blueprints/Habitacion_BP.Habitacion_BP_C" (`KismetMathLibrary.MakeTransform` (`KismetMathLibrary.MakeVector` (+ (.x (`SceneComponent.K2_GetComponentLocation` (`self.PaperSprite22`))) 64.0) (.y (`SceneComponent.K2_GetComponentLocation` (`self.PaperSprite22`))) (.z (`SceneComponent.K2_GetComponentLocation` (`self.PaperSprite22`))))) "Undefined" "OverrideRootScale" null null)
  (`KismetSystemLibrary.PrintString` "Habitacion Generada")
  (`ActorComponent.K2_DestroyComponent` (`self.Box`)))

(fn `UserConstructionScript`)