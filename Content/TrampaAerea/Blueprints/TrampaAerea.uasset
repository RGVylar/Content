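; Aerial trap actor for a 2D side-scroller that moves along a path and eliminates what touches it.
; On BeginPlay, a timeline lerps the PaperSprite's world location between the Inicio and Fin components.
; Overlapping the Box sets End on the player's 2DSideScrollerCharacter and hides the player, while any other overlapping actor is destroyed.
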(event `self.ReceiveBeginPlay`
  (bind (_direction _newtrack_0) (`Timeline|Timeline_0`)
    (:`Update`
      (`SceneComponent.K2_SetWorldLocation` (`self.PaperSprite`) (`KismetMathLibrary.VLerp` (`SceneComponent.K2_GetComponentLocation` (`self.Inicio`)) (`SceneComponent.K2_GetComponentLocation` (`self.Fin`)) _newtrack_0) false false))))

(event `self.Box.OnComponentBeginOverlap`
  (params (OverlappedComponent :type "PrimitiveComponent Object Reference") (OtherActor :type "Actor Object Reference") (OtherComp :type "PrimitiveComponent Object Reference") (OtherBodyIndex :type Integer) (bFromSweep :type Boolean) (SweepResult :type "HitResult Structure (by ref)"))
  (if (== OtherActor (`GameplayStatics.GetPlayerCharacter` 0))
    (set `/Game/Personaje/Blueprints/2DSideScrollerCharacter.End` true (cast `/Game/Personaje/Blueprints/2DSideScrollerCharacter` (`GameplayStatics.GetPlayerPawn` 0) :!pure true))
    (`self.SetActorHiddenInGame` OtherActor true)
    (else
      (`self.K2_DestroyActor` OtherActor))))

(fn `UserConstructionScript`)