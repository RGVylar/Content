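; Short-lived explosion actor for a 2D side-scroller that ends the game for a player caught in it.
; It destroys itself after a brief delay from BeginPlay.
; While it exists, a box overlap with the player character sets that character's End flag and calls SetActorHiddenInGame with false, leaving it visible.
; A node to destroy the overlapped actor is present but never runs.
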(event `self.ReceiveBeginPlay`
  (`KismetSystemLibrary.Delay` 0.2)
  (`self.K2_DestroyActor`))

(event `self.Box.OnComponentBeginOverlap`
  (params (OverlappedComponent :type "PrimitiveComponent Object Reference") (OtherActor :type "Actor Object Reference") (OtherComp :type "PrimitiveComponent Object Reference") (OtherBodyIndex :type Integer) (bFromSweep :type Boolean) (SweepResult :type "HitResult Structure (by ref)"))
  (bind _as2dside_scroller_character (cast `/Game/Personaje/Blueprints/2DSideScrollerCharacter` (`GameplayStatics.GetPlayerPawn` 0) :!pure true))
  (if (== (`GameplayStatics.GetPlayerCharacter` 0) OtherActor)
    (set `/Game/Personaje/Blueprints/2DSideScrollerCharacter.End` true _as2dside_scroller_character)
    (`self.SetActorHiddenInGame` _as2dside_scroller_character false)
    (`self.SetActorHiddenInGame` OtherActor false)))

(fn `UserConstructionScript`)