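; Teleporter actor for a side-scroller that sends the character from an entrance (Entrada) to an exit (Salida) a limited number of times.
; On overlap, while Rondas is below Objetivo, it moves the 2DSideScrollerCharacter to the exit's Y and Z, keeping its current X.
; Each teleport increments the round counter and shows it on a TextRender; once the target is reached, overlaps do nothing.
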(event `self.Entrada.OnComponentBeginOverlap`
  (params (OverlappedComponent :type "PrimitiveComponent Object Reference") (OtherActor :type "Actor Object Reference") (OtherComp :type "PrimitiveComponent Object Reference") (OtherBodyIndex :type Integer) (bFromSweep :type Boolean) (SweepResult :type "HitResult Structure (by ref)"))
  (if (not (>= (`self.Rondas`) (`self.Objetivo`)))
    (bind _as2dside_scroller_character (cast `/Game/Personaje/Blueprints/2DSideScrollerCharacter` OtherActor))
    (bind _rootcomponent (`Actor.RootComponent` _as2dside_scroller_character))
    (`SceneComponent.K2_SetRelativeLocation` _rootcomponent (`KismetMathLibrary.MakeVector` (.x (`SceneComponent.K2_GetComponentLocation` _rootcomponent)) (.y (`SceneComponent.K2_GetComponentLocation` (`self.Salida`))) (.z (`SceneComponent.K2_GetComponentLocation` (`self.Salida`)))) false false)
    (bind _result (`/Engine/EditorBlueprintResources/StandardMacros.IncrementFloat` (`self.Rondas`))
      (:`  `
        (bind _output_get (set `self.Rondas` _result))
        (`TextRenderComponent.K2_SetText` (`self.TextRender`) (`KismetTextLibrary.Conv_DoubleToText` _output_get "HalfToEven"))))))

(fn `UserConstructionScript`)